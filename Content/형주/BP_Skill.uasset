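; BP_Skill is a short-lived skill actor that fires a radial force impulse when it spawns.
; On BeginPlay it also applies an impulse to its static mesh, but the velocity is multiplied by a zero vector, so that impulse is zero.
; After a five-second delay it spawns a fire burst particle effect at its location and destroys itself.
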(event EventBeginPlay
  (Physics|AddImpulseatLocation (Variables|Default|GetStaticMesh) (* (Transformation|GetVelocity) "0.000000,0.000000,0.000000") (Transformation|GetActorLocation) "None")
  (Class|RadialForceComponent|FireImpulse (Variables|Default|GetRadialForce))
  (Utilities|FlowControl|Delay 5.0)
  (Effects|SpawnEmitteratLocation "/Game/InfinityBladeEffects/Effects/FX_Mobile/Fire/combat/P_DmgField_Fire_Activate_02_Burst.P_DmgField_Fire_Activate_02_Burst" (Transformation|GetActorLocation))
  (Actor|DestroyActor))

(fn ConstructionScript)