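; Floor tile for an endless runner that chains track segments and scatters coins on itself.
; The construction script adds child actor components at random points inside the CoinArea box to spawn the coins.
; When a RunnerChar overlaps EndTrigger, the tile asks RunGameMode to add another tile, then destroys itself after a short delay.
; GetAttachTranform exposes the AttachPoint world transform as a connection point.
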(event OnComponentBeginOverlap(EndTrigger)
  (params (OverlappedComponent :type Primitive%20Component%20Object%20Reference) (OtherActor :type Actor%20Object%20Reference) (OtherComp :type Primitive%20Component%20Object%20Reference) (OtherBodyIndex :type Integer) (bFromSweep :type Boolean) (SweepResult :type Hit%20Result%20Structure%20%28by%20ref%29))
  (Utilities|Casting|CastToRunnerChar OtherActor)
  (bind _asrun_game_mode (Utilities|Casting|CastToRunGameMode (Game|GetGameMode)))
  (Default|AddFloorTile _asrun_game_mode)
  (Utilities|FlowControl|Delay 2.0)
  (Actor|DestroyActor))

(event EventBeginPlay)

(event Collision|EventActorBeginOverlap
  (params (OtherActor :type Actor%20Object%20Reference)))

(fn ConstructionScript
  (CallFunction|SpawnCoins))

(fn SpawnCoins
  (bind _coinarea (Variables|컴포넌트|GetCoinArea))
  (for _index (range 0 2)
    (AddComponent|AddChildActorComponent false (Math|Conversions|ToTransform(Vector) (Math|Random|RandomPointinBoundingBox (Variables|/Script/Engine.SceneComponent|GetRelativeLocation _coinarea) (Variables|/Script/Engine.BoxComponent|GetBoxExtent _coinarea))))))

(fn GetAttachTranform
  (return (Transformation|GetWorldTransform (Variables|컴포넌트|GetAttachPoint))))